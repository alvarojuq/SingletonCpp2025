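; BP_MoveActorCommand is a move command that shifts a target actor when executed.
; Execute teleport-free and without sweep offsets TargetActor by a fixed step along world X, then zeroes the NewLocation variable.
; Undo logic, saving of OldLocation, a move to NewLocation and debug prints exist only as disconnected nodes, so the move cannot be reverted.
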(event EventBeginPlay)

(event Collision|EventActorBeginOverlap
  (params (OtherActor :type Actor%20Object%20Reference)))

(event EventTick
  (params (DeltaSeconds :type Float%20%28single-precision%29)))

(event EventExecute
  (bind _targetactor (Variables|Default|GetTargetActor))
  (Transformation|SetActorLocation _targetactor (+ (Transformation|GetActorLocation _targetactor) (Math|Vector|MakeVector 1e+02 0.0 0.0)) false false)
  (Variables|Default|SetNewLocation "0, 0, 0"))

(fn ConstructionScript)