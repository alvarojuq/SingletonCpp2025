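; Command-pattern invoker Blueprint that runs whichever command it currently holds by calling ExecuteMessage on it.
; The InvokeCommand event converts CurrentCommand to an object, while the InvokeCommandAction function uses CurrentCommandObj directly; both check validity before executing.
; Both paths print a debug message when fired, but only the function reports a missing command.
; Neither command variable is assigned within these graphs.
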(event Custom|InvokeCommand
  (bind _currentcommand (Variables|Default|GetCurrentCommand))
  (bind _returnvalue (Utilities|ToObject(Interface) _currentcommand))
  (Development|PrintString "Invoke fired")
  (Utilities|IsValid _returnvalue
    (:Is%20Valid
      (Class|BPICommand|Execute(Message) _returnvalue))))

(event EventBeginPlay)

(event Collision|EventActorBeginOverlap
  (params (OtherActor :type Actor%20Object%20Reference)))

(event EventTick
  (params (DeltaSeconds :type Float%20%28single-precision%29)))

(fn ConstructionScript)

(fn InvokeCommandAction
  (Development|PrintString "Invoke fired")
  (Utilities|IsValid (Variables|Default|GetCurrentCommandObj)
    (:Is%20Valid
      (Class|BPICommand|Execute(Message) (Variables|Default|GetCurrentCommandObj)))
    (:Is%20Not%20Valid
      (Development|PrintString "No Command set"))))