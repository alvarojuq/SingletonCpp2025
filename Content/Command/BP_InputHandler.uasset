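; BP_InputHandler is an input actor for a command-pattern setup that moves an assigned actor and requests undo.
; On BeginPlay it caches the first BP_CommandManager found.
; M spawns a BP_MoveActorCommand targeting ActorToMove at the world origin, clears the manager reference, then executes the command directly.
; Z calls UndoMessage on the manager if valid, so it only prints "Null" once M has run; debug prints trace each step.
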(event EventBeginPlay
  (Development|PrintString "BP_InputHandler BeginPlay")
  (bind _outactors (Actor|GetAllActorsOfClass "/Game/Command/BP_CommandManager.BP_CommandManager_C"))
  (Variables|Default|SetCommandManagerRef (Utilities|Array|Get(acopy) _outactors))
  (Development|PrintString (Utilities|String|Append "\"CommandManagerRef Set To: \"" (Utilities|GetDisplayName (Variables|Default|GetCommandManagerRef)))))

(event Collision|EventActorBeginOverlap
  (params (OtherActor :type Actor%20Object%20Reference)))

(event EventTick
  (params (DeltaSeconds :type Float%20%28single-precision%29)))

(event Input|KeyboardEvents|M
  (params (Key :type Key%20Structure :default "None"))
  (bind _actortomove (Variables|Default|GetActorToMove))
  (:Pressed
    (Development|PrintString "M")
    (bind _returnvalue (Game|SpawnActorfromClass "/Game/Command/BP_MoveActorCommand.BP_MoveActorCommand_C" (Math|Transform|MakeTransform "0, 0, 0") "Undefined" "MultiplyWithRoot" 0 0 "0.000000,0.000000,0.000000" 0))
    (Development|PrintString "command created")
    (bind _asbp_move_actor_command (Utilities|Casting|CastToBP_MoveActorCommand _returnvalue))
    (Variables|/Game/Command/BP_MoveActorCommand.BP_MoveActorCommand_C|SetTargetActor _asbp_move_actor_command _actortomove)
    (Development|PrintString (Utilities|GetDisplayName _actortomove))
    (Variables|/Game/Command/BP_MoveActorCommand.BP_MoveActorCommand_C|SetNewLocation _asbp_move_actor_command "0, 0, 0")
    (Development|PrintString (Utilities|String|Append "\"Calling Execute on: \" +" (Utilities|GetDisplayName _actortomove)))
    (Variables|Default|SetCommandManagerRef 0)
    (Default|Execute _returnvalue)
    (Development|PrintString "ExecuteCommand Called")))

(event Input|KeyboardEvents|Z
  (params (Key :type Key%20Structure :default "None"))
  (bind _commandmanagerref (Variables|Default|GetCommandManagerRef))
  (:Pressed
    (Development|PrintString "Z")
    (Utilities|IsValid _commandmanagerref
      (:Is%20Valid
        (Class|BPICommand|Undo(Message) _commandmanagerref)
        (Development|PrintString "Pressed Z - Undo called"))
      (:Is%20Not%20Valid
        (Development|PrintString "Null")))))

(event Input|KeyboardEvents|Y
  (params (Key :type Key%20Structure :default "None")))

(fn ConstructionScript)