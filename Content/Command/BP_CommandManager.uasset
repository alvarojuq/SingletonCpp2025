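; BP_CommandManager is a command-pattern manager that runs commands and reverses them through an undo stack.
; RunCommandInternal calls Execute on a command, then adds to UndoStack, though the Add shows no connected item.
; The Undo event calls UndoInternal, which undoes and removes the last stack entry, with debug prints throughout.
; Redo is an empty stub with disconnected RedoStack logic, and the Execute event does nothing.
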(event EventBeginPlay)

(event Collision|EventActorBeginOverlap
  (params (OtherActor :type Actor%20Object%20Reference)))

(event EventTick
  (params (DeltaSeconds :type Float%20%28single-precision%29)))

(event EventExecute)

(event EventUndo
  (CallFunction|UndoInternal)
  (Development|PrintString "Undo Internal Called"))

(fn ConstructionScript)

(fn RunCommandInternal
  (params (Command :type BP%20Command%20Manager%20Object%20Reference))
  (Development|PrintString "ExecuteCommand Called")
  (Default|Execute Command)
  (Utilities|Array|Add (Variables|Default|GetUndoStack) 0))

(fn UndoInternal
  (bind _undostack (Variables|Default|GetUndoStack))
  (bind _undostack_2 (Variables|Default|GetUndoStack))
  (bind _undostack_3 (Variables|Default|GetUndoStack))
  (bind _returnvalue (Utilities|Array|LastIndex _undostack_2))
  (bind _returnvalue_2 (Utilities|Array|Length _undostack))
  (Development|PrintString (Utilities|String|ToString(Integer) _returnvalue_2))
  (if (> _returnvalue_2 0)
    (Development|PrintString "Undo function triggered!")
    (bind _output_get (Variables|Default|SetLastUndoCommand (Utilities|Array|Get(acopy) _undostack_3 _returnvalue)))
    (Default|Undo _output_get)
    (Utilities|Array|RemoveIndex _undostack_3 _returnvalue)
    (else
      (Development|PrintString "Nothing to undo"))))

(fn Redo)