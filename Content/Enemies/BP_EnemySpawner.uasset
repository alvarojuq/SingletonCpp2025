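; BP_EnemySpawner is an actor that spawns an enemy and sends it into attack.
; EnemySpawnerEvent spawns EnemyClass slightly above the spawner's location, ignoring collision, then casts the result to BP_Enemy2 and calls Attack on it.
; Debug prints trace the flow, and a second custom event only prints a message.
; BeginPlay, overlap and Tick are empty, so spawning happens only when EnemySpawnerEvent is called.
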(event Custom|CustomEvent
  (Development|PrintString "SpawnEnemyEvent called"))

(event Custom|EnemySpawnerEvent
  (Development|PrintString "Entered BP_EnemySpawner → EnemySpawnerEvent")
  (Utilities|FlowControl|Sequence
    (:then_0
      (Development|PrintString "SpawnEnemyEvent started"))
    (:then_1
      (bind _returnvalue (Game|SpawnActorfromClass (Variables|Default|GetEnemyClass) (Math|Transform|MakeTransform (+ (Transformation|GetActorLocation) (Math|Vector|MakeVector 0.0 0.0 1e+02))) "AlwaysSpawn" "MultiplyWithRoot" 0 0))
      (bind _asbp_enemy_2 (Utilities|Casting|CastToBP_Enemy2 _returnvalue))
      (Default|Attack _asbp_enemy_2))))

(event EventBeginPlay)

(event Collision|EventActorBeginOverlap
  (params (OtherActor :type Actor%20Object%20Reference)))

(event EventTick
  (params (DeltaSeconds :type Float%20%28single-precision%29)))

(fn ConstructionScript)